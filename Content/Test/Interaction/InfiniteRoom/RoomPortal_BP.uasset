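; RoomPortal_BP is a test portal that shows a linked view through a scene capture and teleports the player on contact.
; Each tick, the SceneCapture2D mirrors the player camera's offset and rotation, transformed by the Imagesource component's relative transform.
; An ImagePlane overlap moves the player pawn relative to Imagesource and adjusts control rotation.
; Automatic render target resizing is only stubbed.
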(event `self.ReceiveBeginPlay`
  ;[1 0.08854 0.8757] AUTOMATIC RENDER TARGET RESOLUTION
)

(event `self.ReceiveTick`
  (params (DeltaSeconds :type "Float (single-precision)"))
  ;[0.1765 0.1765 0.1765] SCENE CAPTURE 2D | POSTION - ROTATION
  (`SceneComponent.K2_SetRelativeLocationAndRotation` (`self.SceneCaptureComponent2D`) (+ (`SceneComponent.RelativeLocation` (`self.Imagesource`)) (`KismetMathLibrary.GreaterGreater_VectorRotator` (- (`PlayerCameraManager.GetCameraLocation` (`GameplayStatics.GetPlayerCameraManager` 0)) (`self.K2_GetActorLocation`)) (`KismetMathLibrary.NegateRotator` (`SceneComponent.RelativeRotation` (`self.Imagesource`))))) (`KismetMathLibrary.ComposeRotators` (`PlayerCameraManager.GetCameraRotation` (`GameplayStatics.GetPlayerCameraManager` 0)) (`KismetMathLibrary.NegateRotator` (`SceneComponent.RelativeRotation` (`self.Imagesource`)))) false false))

(event `self.ImagePlane.OnComponentBeginOverlap`
  (params (OverlappedComponent :type "PrimitiveComponent Object Reference") (OtherActor :type "Actor Object Reference") (OtherComp :type "PrimitiveComponent Object Reference") (OtherBodyIndex :type Integer) (bFromSweep :type Boolean) (SweepResult :type "HitResult Structure (by ref)"))
  ;[0.1765 0.1765 0.1765] TELEPORTATION
  (`self.K2_SetActorLocation` (`GameplayStatics.GetPlayerPawn` 0) (+ (`SceneComponent.K2_GetComponentLocation` (`self.Imagesource`)) (`KismetMathLibrary.GreaterGreater_VectorRotator` (- (`.Location` (`GameplayStatics.BreakHitResult` SweepResult)) (`SceneComponent.K2_GetComponentLocation` (`self.DefaultSceneRoot`))) (`KismetMathLibrary.NegateRotator` (`SceneComponent.RelativeRotation` (`self.Imagesource`))))) false false)
  (`Controller.SetControlRotation` (`Pawn.GetController` (`GameplayStatics.GetPlayerPawn` 0)) (`KismetMathLibrary.ComposeRotators` (`PlayerCameraManager.GetCameraRotation` (`GameplayStatics.GetPlayerCameraManager` 0)) (`KismetMathLibrary.NegateRotator` (`SceneComponent.K2_GetComponentRotation` (`self.Imagesource`))))))

(fn `UserConstructionScript`)